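; Player controller for a TPS that owns the main HUD and drives the player's death and respawn flow.
; BeginPlay creates MainWindow and caches the MainCharacter1 pawn, then Tick pushes its HP and weapon-name or "activate" interaction prompt to the widget.
; When HP runs out, Tick shows game over with UI-only input.
; Restart spawns and possesses a new character at the first PlayerStart found, restoring game input.
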(event `self.ReceiveBeginPlay`
  (`|ExecutionSequence`
    (:`then_0`
      (bind _returnvalue (`|CreateWidget` "/Game/JohnnyYegorTPS/UIX/MainWindow.MainWindow_C"))
      (set `self.MainWindow` _returnvalue)
      (`UserWidget.AddToViewport` (`self.MainWindow`) 0))
    (:`then_1`
      (bind _asmain_character_1 (cast `/Game/JohnnyYegorTPS/BluePrints/Character/MainCharacter1` (`self.K2_GetPawn`)))
      (set `self.MyPawnRef` _asmain_character_1))))

(event `self.ReceiveTick`
  (params (DeltaSeconds :type "Float (single-precision)"))
  (bind _mypawnref (`self.MyPawnRef`))
  (if (`KismetSystemLibrary.IsValid` (`self.MyPawnRef`))
    (`|ExecutionSequence`
      (:`then_0`
        (`/Game/JohnnyYegorTPS/UIX/MainWindow.UpdateHPInfo` (`self.MainWindow`) (`/Game/JohnnyYegorTPS/BluePrints/Character/MainCharacter1.HPCurrent` _mypawnref) (`/Game/JohnnyYegorTPS/BluePrints/Character/MainCharacter1.HPMax(Const)` _mypawnref)))
      (:`then_1`
        (if (`KismetSystemLibrary.IsValid` (`/Game/JohnnyYegorTPS/BluePrints/Character/MainCharacter1.WeaponRefInteract` (`self.MyPawnRef`)))
          (`/Game/JohnnyYegorTPS/UIX/MainWindow.UpdateInteractInfo` (`self.MainWindow`) (`KismetTextLibrary.Conv_NameToText` (`/Game/JohnnyYegorTPS/BluePrints/Weapon/BaseWeapon.WeaponName` (`/Game/JohnnyYegorTPS/BluePrints/Character/MainCharacter1.WeaponRefInteract` (`self.MyPawnRef`)))))
          (elif (`KismetSystemLibrary.IsValid` (`/Game/JohnnyYegorTPS/BluePrints/Character/MainCharacter1.IntractReference` (`self.MyPawnRef`)))
            (`/Game/JohnnyYegorTPS/UIX/MainWindow.UpdateInteractInfo` (`self.MainWindow`) "activate")
            (else
              (`/Game/JohnnyYegorTPS/UIX/MainWindow.UpdateInteractInfo` (`self.MainWindow`) "")))))
      (:`then_2`
        (if (`self.Alive`)
          (if (<= (`/Game/JohnnyYegorTPS/BluePrints/Character/MainCharacter1.HPCurrent` (`self.MyPawnRef`)) 0.0)
            (set `self.Alive` false)
            (`/Game/JohnnyYegorTPS/UIX/MainWindow.Game Over` (`self.MainWindow`))
            (set `self.bShowMouseCursor` true)
            (`WidgetBlueprintLibrary.SetInputMode_UIOnlyEx` self (`self.MainWindow`))))))))

(event `Restart`
  (`WidgetSwitcher.SetActiveWidgetIndex` (`/Game/JohnnyYegorTPS/UIX/MainWindow.MainSwitcher` (`self.MainWindow`)) 0)
  (bind _outactors (`GameplayStatics.GetAllActorsOfClass` "/Script/Engine.PlayerStart"))
  (bind _returnvalue (`|SpawnActorFromClass` "/Game/JohnnyYegorTPS/BluePrints/Character/MainCharacter1.MainCharacter1_C" (`self.GetTransform` (`|GetArrayItem` _outactors)) "AlwaysSpawn" "OverrideRootScale" null null))
  (set `self.MyPawnRef` _returnvalue)
  (`self.UnPossess`)
  (`self.Possess` (`self.MyPawnRef`))
  (`WidgetBlueprintLibrary.SetInputMode_GameOnly` self)
  (set `self.Alive` true)
  (set `self.bShowMouseCursor` false))

(fn `UserConstructionScript`)