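; VoidZone is a damage-over-time area that hurts any actor inside its box volume.
; Box overlap begin and end events add and remove actors in a MyTargets array, with no filtering by type.
; Each Tick applies damage to every tracked target, scaling DamagePerSeconds by delta time for a frame-rate-independent rate.
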(event `self.ReceiveTick`
  (params (DeltaSeconds :type "Float (single-precision)"))
  (if (> (`KismetArrayLibrary.Array_Length` (`self.MyTargets`)) 0)
    (for _array_element (`self.MyTargets`)
      (`GameplayStatics.ApplyDamage` _array_element (* DeltaSeconds (`self.DamagePerSeconds`))))))

(event `self.Box.OnComponentBeginOverlap`
  (params (OverlappedComponent :type "PrimitiveComponent Object Reference") (OtherActor :type "Actor Object Reference") (OtherComp :type "PrimitiveComponent Object Reference") (OtherBodyIndex :type Integer) (bFromSweep :type Boolean) (SweepResult :type "HitResult Structure (by ref)"))
  (`KismetArrayLibrary.Array_Add` (`self.MyTargets`) OtherActor))

(event `self.Box.OnComponentEndOverlap`
  (params (OverlappedComponent :type "PrimitiveComponent Object Reference") (OtherActor :type "Actor Object Reference") (OtherComp :type "PrimitiveComponent Object Reference") (OtherBodyIndex :type Integer))
  (`KismetArrayLibrary.Array_RemoveItem` (`self.MyTargets`) OtherActor))

(fn `UserConstructionScript`)