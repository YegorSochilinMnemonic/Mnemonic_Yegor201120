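; Interactable elevator Blueprint that moves its static mesh along a spline path when activated.
; ActivateInteract calls the parent handler, then passes its flag to ElevatorStart.
; ElevatorStart plays the ElevatorMovie timeline when the flag is true and reverses it otherwise.
; Each timeline update sets the mesh's world location from the spline at the Scale time value.
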(event `self.ActivateInteract`
  (params (ActivateInteract :type Boolean))
  (`parent.ActivateInteract` ActivateInteract)
  (`self.ElevatorStart` ActivateInteract))

(event `ElevatorStart`
  (params (StartStop :type Boolean))
  (bind _output_get (set `self.Start/Stop` StartStop))
  (if _output_get
    (bind (_direction _scale) (`Timeline|ElevatorMovie` :!label _label)
      (:`Update`
        (`SceneComponent.K2_SetWorldLocation` (`self.StaticMesh`) (`SplineComponent.GetLocationAtTime` (`self.Spline`) _scale "World" false) false false)))
    (else
      (goto _label :!via `Reverse`))))

(fn `UserConstructionScript`
  (`parent.UserConstructionScript`))