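; Laser gun weapon Blueprint that deals continuous hitscan damage while firing.
; FireBaseWeapon sets an active flag, and Tick then line-traces by object type forward from the shell spawn point over the weapon's range.
; Hits apply damage scaled by frame time and move an impact particle to the hit point with looping-style audio control; misses or inactivity deactivate both.
; The only visible beam here is the trace's one-frame debug line.
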(event `self.FireBaseWeapon`
  (params (Activate :type Boolean))
  (set `self.IsActive` Activate))

(event `self.ReceiveTick`
  (params (DeltaSeconds :type "Float (single-precision)"))
  (bind _audio (`self.Audio`))
  (bind _returnvalue (`SceneComponent.K2_GetComponentLocation` (`self.SpawnShellPlace`)))
  (`parent.ReceiveTick` DeltaSeconds)
  (if (`self.IsActive`)
    (`ActorComponent.Activate` _audio false)
    (bind (_outhit _returnvalue_2) (`KismetSystemLibrary.LineTraceSingleForObjects` :`Start` _returnvalue :`End` (+ _returnvalue (* (`SceneComponent.GetForwardVector` (`self.SpawnShellPlace`)) (`self.Distance`))) :`ObjectTypes` (`|MakeArray` "ObjectTypeQuery1" "ObjectTypeQuery3" "ObjectTypeQuery4" "ObjectTypeQuery5" "ObjectTypeQuery6" :!type "EObjectTypeQuery Enum") :`DrawDebugType` "ForOneFrame"))
    (if _returnvalue_2
      (`ActorComponent.Activate` (`self.ParticleSystem`) false)
      (`ActorComponent.Activate` (`self.Audio`) false)
      (bind (_bblockinghit _binitialoverlap _time _distance _location _impactpoint _normal _impactnormal _physmat _hitactor) (`GameplayStatics.BreakHitResult` _outhit))
      (`GameplayStatics.ApplyDamage` _hitactor (* (`self.WeaponDamage`) (`GameplayStatics.GetWorldDeltaSeconds`)))
      (`SceneComponent.K2_SetWorldLocation` (`self.ParticleSystem`) _location false false)
      (else
        (`ActorComponent.Deactivate` (`self.ParticleSystem`))
        (`ActorComponent.Deactivate` (`self.Audio`))))
    (else
      (`ActorComponent.Deactivate` (`self.ParticleSystem`))
      (`ActorComponent.Deactivate` _audio))))

(fn `UserConstructionScript`
  (`parent.UserConstructionScript`))