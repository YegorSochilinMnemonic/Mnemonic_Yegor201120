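; AI controller for third-person shooter bots that patrol, spot opposing-team characters and attack them.
; On possess it equips the pawn with a random weapon and gathers patrol points from the pawn, falling back to all target points in the level.
; AI Perception sets or clears the enemy and focus.
; Tick chooses between timed firing within range, chasing when farther away, and random patrol with pauses when no enemy exists.
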(event `self.ReceivePossess`
  (params (PossessedPawn :type "Pawn Object Reference"))
  (bind _mycontrolledpawn (`self.MyControlledPawn`))
  (bind _weaponarray (`self.WeaponArray`))
  (bind _asai_character (cast `/Game/JohnnyYegorTPS/BluePrints/AI/AI_Character` (`self.K2_GetPawn`)))
  (set `self.MyControlledPawn` _asai_character)
  (bind _returnvalue (`|SpawnActorFromClass` (`|GetArrayItem` _weaponarray (`KismetMathLibrary.RandomIntegerInRange` 0 (`KismetArrayLibrary.Array_LastIndex` _weaponarray))) (`self.GetTransform` (`self.MyControlledPawn`)) "AlwaysSpawn" "OverrideRootScale" null null))
  (set `/Game/JohnnyYegorTPS/BluePrints/Character/MainCharacter1.WeaponRefInteract` _returnvalue _mycontrolledpawn)
  (`/Game/JohnnyYegorTPS/BluePrints/Character/MainCharacter1.TakeItem` _mycontrolledpawn)
  (if (> (`KismetArrayLibrary.Array_Length` (`/Game/JohnnyYegorTPS/BluePrints/AI/AI_Character.MyTP` (`self.MyControlledPawn`))) 0)
    (set `self.MyTP` (`/Game/JohnnyYegorTPS/BluePrints/AI/AI_Character.MyTP` (`self.MyControlledPawn`)))
    (else
      (bind _outactors (`GameplayStatics.GetAllActorsOfClass` "/Game/JohnnyYegorTPS/BluePrints/AI/MyTargetPoint.MyTargetPoint_C"))
      (set `self.MyTP` _outactors))))

(event `MoveToTP`
  (bind _mytp (`self.MyTP`))
  ;[1 1 1] Патрулирование
  (if (not (`self.OnPatrol`))
    (set `self.OnPatrol` true)
    (`|AIMoveTo` (`self.MyControlledPawn`) (0.0 0.0 0.0) (`|GetArrayItem` _mytp (`KismetMathLibrary.RandomIntegerInRange` 0 (`KismetArrayLibrary.Array_LastIndex` _mytp))) 64.0
      (:`OnSuccess`
        _)
      (:`OnFail`
        _))
    (`KismetSystemLibrary.Delay` 3.0)
    (set `self.OnPatrol` false)))

(event `ChaseToEnemy`
  ;[1 1 1] Погоня за врагом
  (`|AIMoveTo` (`self.MyControlledPawn`) (0.0 0.0 0.0) (`self.Enemy`) 600.0))

(event `Fire`
  (if (not (`self.OnFire`))
    (set `self.OnFire` true)
    (`/Game/JohnnyYegorTPS/BluePrints/Character/MainCharacter1.Fire` (`self.MyControlledPawn`) true)
    (`KismetSystemLibrary.Delay` 1.2)
    (`/Game/JohnnyYegorTPS/BluePrints/Character/MainCharacter1.Fire` (`self.MyControlledPawn`) true)
    (`KismetSystemLibrary.Delay` 1.0)
    (set `self.OnFire` false)))

(event `self.ReceiveTick`
  (params (DeltaSeconds :type "Float (single-precision)"))
  (set `/Game/JohnnyYegorTPS/BluePrints/Character/MainCharacter1.OnAim` (`KismetSystemLibrary.IsValid` (`self.Enemy`)) (`self.MyControlledPawn`))
  (if (`KismetSystemLibrary.IsValid` (`self.Enemy`))
    (if (< (`self.GetDistanceTo` (`self.MyControlledPawn`) (`self.Enemy`)) (`self.FireDistance`))
      (`self.Fire`)
      (else
        (`self.ChaseToEnemy`)))
    (else
      (`self.MoveToTP`))))

(event `self.AIPerception.OnTargetPerceptionUpdated`
  (params (Actor :type "Actor Object Reference") (Stimulus :type "AIStimulus Structure"))
  (if (`.bSuccessfullySensed` (break `AIStimulus` Stimulus))
    (bind _asmain_character_1 (cast `/Game/JohnnyYegorTPS/BluePrints/Character/MainCharacter1` Actor))
    (if (not (`|EnumEquality` (`/Game/JohnnyYegorTPS/BluePrints/Character/MainCharacter1.MyTeam` _asmain_character_1) (`/Game/JohnnyYegorTPS/BluePrints/Character/MainCharacter1.MyTeam` (`self.MyControlledPawn`))))
      (bind _output_get (set `self.Enemy` _asmain_character_1))
      (`self.K2_SetFocus` _output_get))
    (elif (== Actor (`self.Enemy`))
      (bind _output_get_2 (set `self.Enemy` null))
      (`self.K2_SetFocus` _output_get_2))))

(fn `UserConstructionScript`)